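; GA_LightingSlash is a Gameplay Ability that plays the mage's Lighting Slash cast animation.
; On activation it casts the owner actor to BP_MageCharacter, stores the reference and commits the ability, cancelling if either step fails.
; It then plays AM_CastLightingSlash on the character mesh and ends when the montage completes, blends out or is interrupted.
; The graph itself contains no damage or effect logic.
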(event Ability|EventActivateAbility
  (bind _asbp_mage_character (Utilities|Casting|CastToBP_MageCharacter (.OwnerActor (Utilities|Struct|BreakGameplayAbilityActorInfo (Ability|GetActorInfo))))
    (:then
      (Variables|Default|SetMageCharacterReference _asbp_mage_character)
      (bind _returnvalue (Ability|CommitAbility))
      (if _returnvalue
        (Animation|Montage|PlayMontage (Variables|/Script/Engine.Character|GetMesh (Variables|Default|GetMageCharacterReference)) "/Game/Blueprints/Characters/Mage/Animations/AM_CastLightingSlash.AM_CastLightingSlash"
          (:OnCompleted
            _)
          (:OnBlendOut
            _)
          (:OnInterrupted
            _))
        (Ability|EndAbility)
        (else
          (Ability|CancelAbility :!label _label))))
    (:CastFailed
      (goto _label))))

(event Ability|EventOnEndAbility
  (params (bWasCancelled :type Boolean)))