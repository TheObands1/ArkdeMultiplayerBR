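; Gameplay ability that casts a firebolt for the mage character.
; After committing, it plays the cast montage and, on a notify, spawns a firebolt projectile moved to the right-hand socket.
; The projectile launches along the mage's forward vector, with the caster's current speed added to its own.
; Montage completion, blend-out or interruption ends the ability, while a failed cast to the mage or failed commit cancels it.
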(event Ability|EventActivateAbility
  (bind _asbp_mage_character (Utilities|Casting|CastToBP_MageCharacter (.OwnerActor (Utilities|Struct|BreakGameplayAbilityActorInfo (Ability|GetActorInfo))))
    (:then
      (Variables|Default|SetMageCharacterReference _asbp_mage_character)
      (bind _returnvalue (Ability|CommitAbility))
      (if _returnvalue
        (Animation|Montage|PlayMontage (Variables|/Script/Engine.Character|GetMesh (Variables|Default|GetMageCharacterReference)) "/Game/Blueprints/Characters/Mage/Animations/AM_CastFirebolt.AM_CastFirebolt"
          (:OnCompleted
            (Ability|EndAbility :!label _label))
          (:OnBlendOut
            (goto _label))
          (:OnInterrupted
            (goto _label))
          (:OnNotifyBegin
            (bind _spawnedactor (|SpawnActor :Class "/Game/Blueprints/Abilities/Firebolt/BP_FireboltProjectile.BP_FireboltProjectile_C" :Instigator (Variables|Default|GetMageCharacterReference))
              (:Success
                (bind _asbp_firebolt_projectile (Utilities|Casting|CastToBP_FireboltProjectile _spawnedactor))
                (bind _output_get (Variables|Default|SetFireboltProjectileReference _asbp_firebolt_projectile))
                (Transformation|SetActorLocation _output_get (Transformation|GetSocketLocation (Variables|/Script/Engine.Character|GetMesh (Variables|Default|GetMageCharacterReference)) "AbilityRightHandSocket") false false)
                (Class|BRProjectile|InitializeProjectileMovement (Variables|Default|GetFireboltProjectileReference) (* (Transformation|GetActorForwardVector (Variables|Default|GetMageCharacterReference)) (+ (Variables|Default|GetProjectileSpeed) (Math|Vector|VectorLength (Transformation|GetVelocity (Variables|Default|GetMageCharacterReference))))))))))
        (else
          (Ability|CancelAbility :!label _label_2))))
    (:CastFailed
      (goto _label_2))))

(event Ability|EventOnEndAbility
  (params (bWasCancelled :type Boolean)))