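; BP_Storm is the battle royale storm zone, a circle that resizes over time and damages characters outside it.
; On the authority, a timeline paced by ScalingTime lerps StormCircle's X and Y scale between MinScale and MaxScale while Z stays at MaxScale.
; Leaving the circle applies GE_StormDamage through the BattleRoyaleCharacter's Ability System Component, and re-entering removes all its stacks, also server-side only.
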(event OnComponentBeginOverlap(StormCircle)
  (params (OverlappedComponent :type Primitive%20Component%20Object%20Reference) (OtherActor :type Actor%20Object%20Reference) (OtherComp :type Primitive%20Component%20Object%20Reference) (OtherBodyIndex :type Integer) (bFromSweep :type Boolean) (SweepResult :type Hit%20Result%20Structure%20%28by%20ref%29))
  (Networking|SwitchHasAuthority
    (:Authority
      (bind _asbattle_royale_character (Utilities|Casting|CastToBattleRoyaleCharacter OtherActor))
      (Utilities|IsValid (Variables|/Script/BattleRoyale.BattleRoyaleCharacter|GetAbilitySystemComponent _asbattle_royale_character)
        (:Is%20Valid
          (GameplayEffects|RemoveActiveGameplayEffectbySourceEffect (Variables|/Script/BattleRoyale.BattleRoyaleCharacter|GetAbilitySystemComponent _asbattle_royale_character) "/Game/Blueprints/Abilities/Storm/GE_StormDamage.GE_StormDamage_C" 0 -1))))))

(event OnComponentEndOverlap(StormCircle)
  (params (OverlappedComponent :type Primitive%20Component%20Object%20Reference) (OtherActor :type Actor%20Object%20Reference) (OtherComp :type Primitive%20Component%20Object%20Reference) (OtherBodyIndex :type Integer))
  (Networking|SwitchHasAuthority
    (:Authority
      (bind _asbattle_royale_character (Utilities|Casting|CastToBattleRoyaleCharacter OtherActor))
      (Utilities|IsValid (Variables|/Script/BattleRoyale.BattleRoyaleCharacter|GetAbilitySystemComponent _asbattle_royale_character)
        (:Is%20Valid
          (GameplayEffects|ApplyGameplayEffectToSelf :self (Variables|/Script/BattleRoyale.BattleRoyaleCharacter|GetAbilitySystemComponent _asbattle_royale_character) :GameplayEffectClass "/Game/Blueprints/Abilities/Storm/GE_StormDamage.GE_StormDamage_C"))))))

(event EventBeginPlay
  (Networking|SwitchHasAuthority
    (:Authority
      (Components|Timeline|SetPlayRate (Variables|Default|GetStorm_Change) (/ 1.0 (Variables|Default|GetScalingTime)))
      (bind _size_manager (Timeline|Storm_Change Play)
        (:Update
          (Transformation|SetWorldScale3D (Variables|Default|GetStormCircle) (Math|Vector|MakeVector (Math|Float|Lerp (Variables|Default|GetMinScale) (Variables|Default|GetMaxScale) _size_manager) (Math|Float|Lerp (Variables|Default|GetMinScale) (Variables|Default|GetMaxScale) _size_manager) (Variables|Default|GetMaxScale))))))))

(fn ConstructionScript)